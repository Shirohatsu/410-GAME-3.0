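; Player controller for the inventory and crafting system, owning the player's HUD and menu input.
; On BeginPlay it caches the player character and, for the local controller, creates WBP_PlayerHUD with the inventory system and adds the Enhanced Input mapping context.
; Input actions open the inventory and crafting menus through the HUD.
; Helper events spawn alert widgets and forward show/hide message calls to chests, dropped items and normal items.
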(event Custom|CHESTHideMesage
  (params (Item :type Chest%20Object%20Reference))
  ;[1 0.7599 0] Chest show/hide widget
  (Default|HideMesage Item))

(event Custom|ITEMHideMesage2
  (params (Item :type BP%20Item%20Object%20Reference))
  ;[1 0.7599 0] Normal Item show/hide widget
  (Utilities|IsValid Item
    (:Is%20Valid
      (Default|HideMesage Item))))

(event Custom|SetCharacter
  (params (Character :type Character%20Object%20Reference))
  (Variables|Default|SetCharacterForLocation Character))

(event Custom|Add%20ALERT
  (params (Alert%20Text :type Text))
  ;[0.1329 0.7682 1] ALERT
  (bind _returnvalue (UserInterface|CreateWidget "/Game/InventoryAndCraftingSystem/ItemChestInventory/UI/WBP_Alert.WBP_Alert_C" (Game|GetPlayerController 0) Alert%20Text))
  (UserInterface|Viewport|AddtoViewport _returnvalue 0))

(event Custom|ITEMShowMesage2
  (params (Item :type BP%20Item%20Object%20Reference))
  ;[1 0.7599 0] Normal Item show/hide widget
  (Utilities|IsValid Item
    (:Is%20Valid
      (Default|ShowMesage Item))))

(event Custom|CHESTShowMesage
  (params (Item :type Chest%20Object%20Reference))
  ;[1 0.7599 0] Chest show/hide widget
  (Default|ShowMesage Item))

(event Custom|ITEMShowMesage
  (params (Item :type BP%20Item%20Dropped%20Object%20Reference))
  ;[1 0.7599 0] Item dropped show/hide widget
  (Utilities|IsValid Item
    (:Is%20Valid
      (Default|ShowMesage Item))))

(event Custom|ITEMHideMesage
  (params (Item :type BP%20Item%20Dropped%20Object%20Reference))
  ;[1 0.7599 0] Item dropped show/hide widget
  (Utilities|IsValid Item
    (:Is%20Valid
      (Default|HideMesage Item))))

(event Input|EnhancedActionEvents|EnhancedInputActionIA_Crafting
  (params (ActionValue :type Boolean) (ElapsedSeconds :type Float%20%28double-precision%29) (TriggeredSeconds :type Float%20%28double-precision%29) (InputAction :type Input%20Action%20Object%20Reference :default "/Game/InventoryAndCraftingSystem/Input/Actions/IA_Crafting.IA_Crafting"))
  ;[1 0.1465 0] INPUT KEYS
  ;;[0 0.1415 1] crafting system
  (:Started
    (Default|DisplayCraftingMenu (Variables|Default|GetHUD) (Variables|Default|GetNEW_Inventory_System))))

(event Input|EnhancedActionEvents|EnhancedInputActionIA_Inventory
  (params (ActionValue :type Boolean) (ElapsedSeconds :type Float%20%28double-precision%29) (TriggeredSeconds :type Float%20%28double-precision%29) (InputAction :type Input%20Action%20Object%20Reference :default "/Game/InventoryAndCraftingSystem/Input/Actions/IA_Inventory.IA_Inventory"))
  ;[1 0.1465 0] INPUT KEYS
  (:Started
    (Default|DisplayPalyerMenu (Variables|Default|GetHUD))))

(event EventBeginPlay
  (bind _returnvalue (Game|GetPlayerController 0))
  (bind _returnvalue_2 (PlayerController|LocalPlayerSubsystems|GetEnhancedInputLocalPlayerSubsystem _returnvalue))
  (CallFunction|SetCharacter (Game|GetPlayerCharacter 0))
  (if (Pawn|IsLocalPlayerController)
    (bind _returnvalue_3 (UserInterface|CreateWidget "/Game/InventoryAndCraftingSystem/ItemChestInventory/Blueprints/ControllerAndHUD/WBP_PlayerHUD.WBP_PlayerHUD_C" 0 (Variables|Default|GetNEW_Inventory_System)))
    (bind _output_get (Variables|Default|SetHUD _returnvalue_3))
    (UserInterface|Viewport|AddtoViewport _output_get 0)
    (Utilities|IsValid _returnvalue_2
      (:Is%20Valid
        (Input|AddMappingContext _returnvalue_2 "/Game/InventoryAndCraftingSystem/Input/IMC_InventoryAndCrafting.IMC_InventoryAndCrafting" 1 "(bIgnoreAllPressedKeysUntilRelease=True,bForceImmediately=False)")))))

(fn ConstructionScript)