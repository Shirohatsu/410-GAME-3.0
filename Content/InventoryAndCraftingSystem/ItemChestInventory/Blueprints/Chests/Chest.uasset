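; Interactive storage chest that opens its InventorySystem as a HUD container and swings open or shut via a timeline.
; Player overlap registers it as interactive and shows a prompt through the controller, only while the Free flag marks it unused.
; Toggling Free records or clears the user and drives the animation.
; Items dropped into BoxDrop are absorbed after a short delay for quantity setup, while the construction script seeds starting contents.
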(event OnComponentBeginOverlap(PlayerCollisionBox)
  (params (OverlappedComponent :type Primitive%20Component%20Object%20Reference) (OtherActor :type Actor%20Object%20Reference) (OtherComp :type Primitive%20Component%20Object%20Reference) (OtherBodyIndex :type Integer) (bFromSweep :type Boolean) (SweepResult :type Hit%20Result%20Structure%20%28by%20ref%29))
  ;[1 1 1] Collision Box
  (if (Variables|Default|GetFree)
    (CallFunction|ItemGOODtoInteract OtherActor)))

(event OnComponentEndOverlap(PlayerCollisionBox)
  (params (OverlappedComponent :type Primitive%20Component%20Object%20Reference) (OtherActor :type Actor%20Object%20Reference) (OtherComp :type Primitive%20Component%20Object%20Reference) (OtherBodyIndex :type Integer))
  ;[1 1 1] Collision Box
  (CallFunction|ItemBADtoInteract OtherActor))

(event OnComponentBeginOverlap(BoxDrop)
  (params (OverlappedComponent :type Primitive%20Component%20Object%20Reference) (OtherActor :type Actor%20Object%20Reference) (OtherComp :type Primitive%20Component%20Object%20Reference) (OtherBodyIndex :type Integer) (bFromSweep :type Boolean) (SweepResult :type Hit%20Result%20Structure%20%28by%20ref%29))
  ;[1 1 1] when you drop an item from player inventory
  (Utilities|FlowControl|Delay 0.2) ; wait until the item quantity is set
  (CallFunction|ItemDropedonChest OtherActor))

(event Custom|HideMesage
  ;[1 1 1] Show "interact" mesage (widget)
  (Rendering|SetVisibility (Variables|Default|GetWidget) false false)
  (Variables|Default|SetEnable%20Interaction? false))

(event Custom|ShowMesage
  ;[1 1 1] Show "interact" mesage (widget)
  (Rendering|SetVisibility (Variables|Default|GetWidget) true false)
  (Variables|Default|SetEnable%20Interaction? true))

(event Custom|serverSHOW
  (params (MyPlayerController :type BP%20My%20Player%20Controller%20Object%20Reference))
  ;[1 1 1] Show "interact" mesage (widget)
  (Default|CHESTShowMesage MyPlayerController self))

(event Custom|Update%20free
  (params (As%20BP%20My%20Player%20Controller :type BP%20My%20Player%20Controller%20Object%20Reference))
  ;[0.9634 1 0.5154] open/close chest
  (CallFunction|ServerSetUser As%20BP%20My%20Player%20Controller)
  (bind _output_get (Variables|Default|SetFree (not (Variables|Default|GetFree))))
  (if _output_get
    (CallFunction|CloseChest)
    (CallFunction|ServerSetUser) ; no one is using now
    (else
      (CallFunction|OpenChest))))

(event Custom|serverHIDE
  (params (MyPlayerController :type BP%20My%20Player%20Controller%20Object%20Reference))
  ;[1 1 1] Show "interact" mesage (widget)
  (Default|CHESTHideMesage MyPlayerController self))

(event Custom|OpenChest
  ;[0.9634 1 0.5154] open/close chest
  (bind _newtrack_0 (Timeline|Timeline Play)
    (:Update
      (Transformation|SetRelativeRotation (Variables|Default|Getroot) (Math|Rotator|Lerp(Rotator) "0.000000,90.000000,0.000000" "0.000000,90.000000,100.000000" _newtrack_0) false false))))

(event Custom|CloseChest
  ;[0.9634 1 0.5154] open/close chest
  (bind _newtrack_0 (Timeline|Timeline Reverse)
    (:Update
      (Transformation|SetRelativeRotation (Variables|Default|Getroot) (Math|Rotator|Lerp(Rotator) "0.000000,90.000000,0.000000" "0.000000,90.000000,100.000000" _newtrack_0) false false))))

(event Custom|Server%20set%20user
  (params (As%20BP%20My%20Player%20Controller :type BP%20My%20Player%20Controller%20Object%20Reference))
  (Variables|Default|SetAs%20BP%20My%20Player%20Controller As%20BP%20My%20Player%20Controller))

(event EventInteract
  (params (PlayerCharacter :type BP%20My%20Player%20Controller%20Object%20Reference))
  (Default|ShowContainer (Variables|/Game/InventoryAndCraftingSystem/ItemChestInventory/Blueprints/ControllerAndHUD/BP_MyPlayerController.BP_MyPlayerController_C|GetHUD PlayerCharacter) (Variables|Default|GetInventory_System) self))

(fn ConstructionScript
  (Variables|/Game/InventoryAndCraftingSystem/ItemChestInventory/Blueprints/AC_Inventory_System.AC_Inventory_System_C|SetInventorySize (Variables|Default|GetInventory_System) (Variables|Default|GetInventory%20Size))
  (CallFunction|SetInventoryContent)
  (Variables|/Game/InventoryAndCraftingSystem/ItemChestInventory/Blueprints/AC_Inventory_System.AC_Inventory_System_C|SetParent%20Name (Variables|Default|GetInventory_System) (Utilities|GetObjectName self)))

(fn ItemGOODtoInteract
  (params (PlayerCharacter :type Actor%20Object%20Reference))
  (bind _asbp_my_player_controller (Utilities|Casting|CastToBP_MyPlayerController (Game|GetInstigatorController PlayerCharacter)))
  (Default|AddInteractiveActor (Variables|/Game/InventoryAndCraftingSystem/ItemChestInventory/Blueprints/ControllerAndHUD/BP_MyPlayerController.BP_MyPlayerController_C|GetNEW_Inventory_System _asbp_my_player_controller) self)
  (CallFunction|ServerSHOW _asbp_my_player_controller))

(fn ItemBADtoInteract
  (params (PlayerCharacter :type Actor%20Object%20Reference))
  (bind _asbp_my_player_controller (Utilities|Casting|CastToBP_MyPlayerController (Game|GetInstigatorController PlayerCharacter)))
  (Default|RemoveInteractiveActor (Variables|/Game/InventoryAndCraftingSystem/ItemChestInventory/Blueprints/ControllerAndHUD/BP_MyPlayerController.BP_MyPlayerController_C|GetNEW_Inventory_System _asbp_my_player_controller) self)
  (CallFunction|ServerHIDE _asbp_my_player_controller))

(fn ItemDropedonChest
  (params (Actor :type Actor%20Object%20Reference))
  (bind _returnvalue (Actor|GetComponentbyClass Actor "/Game/InventoryAndCraftingSystem/ItemChestInventory/Blueprints/AC_ItemDataComponent.AC_ItemDataComponent_C"))
  (Utilities|Casting|CastToBP_ItemDropped Actor)
  (Utilities|IsValid _returnvalue
    (:Is%20Valid
      (Default|AddItemtoChest _returnvalue self)
      (Default|MCUpdate (Variables|Default|GetInventory_System)))))

(fn GetDropLocation
  (return (Transformation|GetWorldLocation (Variables|Drop|GetDropArrow))))

(fn SetInventoryContent
  (Utilities|Array|Clear (Variables|Default|GetContent))
  (for (_array_element _array_index) (Variables|Default|GetInventory%20Content)
    (Utilities|Array|Insert (Variables|Default|GetContent) (Utilities|Struct|MakeF_SlotStruct (.rowname (.ItemName (Utilities|Struct|BreakF_RowNames _array_element))) (.Quantity (Utilities|Struct|BreakF_RowNames _array_element))) _array_index))
  (Variables|/Game/InventoryAndCraftingSystem/ItemChestInventory/Blueprints/AC_Inventory_System.AC_Inventory_System_C|SetContent (Variables|Default|GetInventory_System) (Variables|Default|GetContent)))