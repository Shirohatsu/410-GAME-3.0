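; Basic melee enemy AI that chases the player and punches on reaching them.
; Pawn Sensing sets a seen flag and calls FollowPlayer, which uses AI MoveTo toward player character 0.
; On arrival it plays a punch montage and applies damage immediately, delaying by the montage length before re-enabling attack, though each sighting also resets that flag.
; Tick pushes Health into the health bar widget as a percentage.
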(event OnSeePawn(PawnSensing)
  (params (Pawn :type Pawn%20Object%20Reference))
  (Variables|Default|SetidentifyPlr true)
  (CallFunction|FollowPlayer))

(event Custom|FollowPlayer
  (Variables|Default|SetCanAttack true)
  (if (Variables|Default|GetidentifyPlr)
    (AI|AIMoveTo self "0, 0, 0" (Game|GetPlayerCharacter 0) 1e+02 false
      (:OnSuccess
        (if (Variables|Default|GetCanAttack)
          (Variables|Default|SetCanAttack false)
          (bind _returnvalue (Animation|PlayAnimMontage "/Game/BluePrints/Punching.Punching" 2.0 "None"))
          (Audio|PlaySoundatLocation 0 "0, 0, 0" "0, 0, 0" 1.0 1.0 0.0 0 0 0 0)
          (Game|Damage|ApplyDamage (Game|GetPlayerCharacter 0) 2.0 0 0)
          (Utilities|FlowControl|Delay _returnvalue)
          (Variables|Default|SetCanAttack true))))))

(event EventBeginPlay)

(event Collision|EventActorBeginOverlap
  (params (OtherActor :type Actor%20Object%20Reference)))

(event EventTick
  (params (DeltaSeconds :type Float%20%28single-precision%29))
  (bind _aswb_enemy_health_bar (Utilities|Casting|CastToWB_EnemyHealthBar (UserInterface|GetWidget (Variables|Default|GetHealthBarWidget))))
  (Progress|SetPercent (Variables|/Game/WB_EnemyHealthBar.WB_EnemyHealthBar_C|GetHealthBarEnemy _aswb_enemy_health_bar) (/ (Variables|Default|GetHealth) 1e+02)))

(fn ConstructionScript)